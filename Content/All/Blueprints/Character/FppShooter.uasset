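; First-person shooter character with movement, weapon controls, a local HUD and camera-based aiming.
; Shoot, aim, reload, switch and drop inputs go through server events broadcast to all clients, mostly forwarding to the current weapon.
; Shots add capped camera pitch recoil that recovers on Tick, and opposite-direction key presses cancel that axis' velocity, briefly blocking movement for counter-strafe stops.
; On death, local UI is removed and the server possesses a spectator spawned behind the body.
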(event Custom|RecoverStopper
  ;[1 1 1] 处理急停
  (Utilities|FlowControl|Delay 0.1)
  (Variables|Default|SetStopper 1.0))

(event Custom|Server-OnShootButtonDown
  ;[1 1 1] 射击
  ;;[1 1 1] 服务器通知所有客户端
  (CallFunction|All-OnShootButtonDown))

(event Custom|All-OnAimButtonDown
  ;[1 1 1] 瞄准
  (Default|OnAimButtonDown (CallFunction|GetCurrentWeapon)))

(event Custom|All-DropWeapon
  ;[1 1 1] 扔枪
  (CallFunction|DropWeapon))

(event Custom|All-OnAimButtonUp
  ;[1 1 1] 瞄准
  (Default|OnAimButtonUp (CallFunction|GetCurrentWeapon)))

(event Custom|Server-OnReloadButtonDown
  ;[1 1 1] 上子弹
  (CallFunction|All-OnReloadButtonDown))

(event Custom|Event_OnDie
  (bind _returnvalue (Transformation|GetActorTransform))
  (Utilities|FlowControl|Delay 0.2)
  (bind _returnvalue_2 (Game|SpawnActorfromClass "/Game/All/Blueprints/Character/Spectator.Spectator_C" (Math|Transform|MakeTransform (+ (.location _returnvalue) (* (Transformation|GetActorForwardVector) -4e+02)) (.rotation _returnvalue) (.scale _returnvalue)) "Undefined" 0 0))
  (Pawn|Possess (Pawn|GetController) _returnvalue_2))

(event Custom|Server-OnReloadButtonUp
  ;[1 1 1] 上子弹
  (CallFunction|All-OnReloadButtonUp))

(event Custom|All-OnReloadButtonDown
  ;[1 1 1] 上子弹
  (Default|OnReloadButtonDown (CallFunction|GetCurrentWeapon)))

(event Custom|All-OnReloadButtonUp
  ;[1 1 1] 上子弹
  (Default|OnReloadButtonUp (CallFunction|GetCurrentWeapon)))

(event Custom|Server-OnShootButtonUp
  ;[1 1 1] 射击
  ;;[1 1 1] 服务器通知所有客户端
  (CallFunction|All-OnShootButtonUp))

(event Custom|Server-SwitchWeapon
  (params (Index :type Integer))
  ;[1 1 1] 切枪服务器广播
  (CallFunction|All-SwitchWeapon Index))

(event Custom|All-OnShootButtonDown
  ;[1 1 1] 射击
  ;;[1 1 1] 收到通知后的每个客户端执行方法
  (Default|OnShootButtonDown (CallFunction|GetCurrentWeapon)))

(event Custom|All-SwitchWeapon
  (params (Index :type Integer))
  ;[1 1 1] 切枪服务器广播
  (CallFunction|SwitchWeapon Index true))

(event Custom|All-OnShootButtonUp
  ;[1 1 1] 射击
  ;;[1 1 1] 收到通知后的每个客户端执行方法
  (Default|OnShootButtonUp (CallFunction|GetCurrentWeapon)))

(event Custom|Server-OnAimButtonUp
  ;[1 1 1] 瞄准
  (CallFunction|All-OnAimButtonUp))

(event Custom|Server-OnAimButtonDown
  ;[1 1 1] 瞄准
  (CallFunction|All-OnAimButtonDown))

(event Custom|Server-DropWeapon
  ;[1 1 1] 扔枪
  (CallFunction|All-DropWeapon))

(event EventBeginPlay
  (|CallParentFunction)
  (if (Pawn|IsLocallyControlled)
    (bind _ui (CallFunction|CreateWidgetandAddtoViewport "/Game/All/UI/Crcsshair/ShooterUI.ShooterUI_C"))
    (Variables|Default|SetShooterUI _ui)))

(event Collision|EventActorBeginOverlap
  (params (OtherActor :type Actor%20Object%20Reference)))

(event EventTick
  (params (DeltaSeconds :type Float%20%28single-precision%29))
  ;[1 1 1] 准星回退
  (CallFunction|RecoilDrop DeltaSeconds))

(event Input|ActionEvents|InputActionMoveAction
  (params (Key :type Key%20Structure :default "None"))
  ;[1 1 1] 处理急停
  (:Pressed
    (CallFunction|Stoplmm Key)))

(event Input|ActionEvents|InputActionShoot
  (params (Key :type Key%20Structure :default "None"))
  ;[1 1 1] 射击
  ;;[1 1 1] 通知服务器
  (:Pressed
    (CallFunction|Server-OnShootButtonDown))
  (:Released
    (CallFunction|Server-OnShootButtonUp)))

(event Input|ActionEvents|InputActionAim
  (params (Key :type Key%20Structure :default "None"))
  ;[1 1 1] 瞄准
  (:Pressed
    (CallFunction|Server-OnAimButtonDown))
  (:Released
    (CallFunction|Server-OnAimButtonUp)))

(event Input|ActionEvents|InputActionReload
  (params (Key :type Key%20Structure :default "None"))
  ;[1 1 1] 上子弹
  (:Pressed
    (CallFunction|Server-OnReloadButtonDown))
  (:Released
    (CallFunction|Server-OnReloadButtonUp)))

(event Input|AxisEvents|InputAxisMoveForward
  (params (AxisValue :type Float%20%28single-precision%29))
  (Pawn|Input|AddMovementInput (Math|Vector|GetForwardVector (Transformation|GetActorRotation)) (* AxisValue (Variables|Default|GetStopper)) false))

(event Input|AxisEvents|InputAxisMoveRight
  (params (AxisValue :type Float%20%28single-precision%29))
  (Pawn|Input|AddMovementInput (Math|Vector|GetRightVector (Transformation|GetActorRotation)) (* AxisValue (Variables|Default|GetStopper)) false))

(event Input|AxisEvents|InputAxisTurn
  (params (AxisValue :type Float%20%28single-precision%29))
  (Pawn|Input|AddControllerYawInput AxisValue))

(event Input|AxisEvents|InputAxisLookUp
  (params (AxisValue :type Float%20%28single-precision%29))
  (Transformation|AddRelativeRotation (Variables|Character|GetMesh) (Math|Rotator|MakeRotator (* AxisValue 1.0) 0.0 0.0) false false))

(event Input|KeyboardEvents|1
  (params (Key :type Key%20Structure :default "None"))
  ;[1 1 1] 切枪通知服务器
  (:Pressed
    (CallFunction|Server-SwitchWeapon 1)))

(event Input|KeyboardEvents|2
  (params (Key :type Key%20Structure :default "None"))
  ;[1 1 1] 切枪通知服务器
  (:Pressed
    (CallFunction|Server-SwitchWeapon 2)))

(event Input|KeyboardEvents|3
  (params (Key :type Key%20Structure :default "None"))
  ;[1 1 1] 切枪通知服务器
  (:Pressed
    (CallFunction|Server-SwitchWeapon 3)))

(event Input|KeyboardEvents|G
  (params (Key :type Key%20Structure :default "None"))
  ;[1 1 1] 扔枪
  (:Pressed
    (CallFunction|Server-DropWeapon)))

(event Input|KeyboardEvents|Q
  (params (Key :type Key%20Structure :default "None"))
  ;[1 1 1] 切枪通知服务器
  (:Pressed
    (CallFunction|Server-SwitchWeapon (Variables|Default|GetLastWeaponIndex))))

(fn ConstructionScript
  (|CallParentFunction))

(fn ModifyMesh
  (Transformation|AttachComponentToComponent (Variables|Character|GetMesh) (Variables|Default|GetCamera) "None" "KeepWorld" "KeepWorld" "KeepWorld" true))

(fn GetShootStartPosition
  (return (Transformation|GetWorldLocation (Variables|Default|GetCamera))))

(fn GetShootDirection
  (return (Transformation|GetWorldRotation (Variables|Default|GetCamera))))

(fn OnShootOnce
  (params (Recoil :type Float%20%28single-precision%29))
  (|CallParentFunction 0.0)
  (bind _output_get (LocalVariables|SetTargetCurrentRecoil (Math|Float|Min(Float) (+ (Variables|Default|GetCurrentRecoil) Recoil) (.MaxRecoil (Utilities|Struct|BreakWeaponStructure (Variables|/Game/All/Blueprints/Weapon/Weapon.Weapon_C|GetConfig (CallFunction|GetCurrentWeapon)))))))
  (Transformation|AddRelativeRotation (Variables|Default|GetCamera) (Math|Rotator|MakeRotator 0.0 (- _output_get (Variables|Default|GetCurrentRecoil)) 0.0) false false)
  (Variables|Default|SetCurrentRecoil (LocalVariables|GetTargetCurrentRecoil)))

(fn RecoilDrop
  (params (Time :type Float%20%28single-precision%29))
  (bind _weapon (CallFunction|GetCurrentWeapon))
  (if (!= (CallFunction|GetCurrentWeapon) 0)
    (if (> (Variables|Default|GetCurrentRecoil) 0.0)
      (Transformation|AddRelativeRotation (Variables|Default|GetCamera) (Math|Rotator|MakeRotator 0.0 (- (Math|Interpolation|FInterptoConstant (Variables|Default|GetCurrentRecoil) 0.0 Time (.RecoilDropSpeed (Utilities|Struct|BreakWeaponStructure (Variables|/Game/All/Blueprints/Weapon/Weapon.Weapon_C|GetConfig _weapon)))) (Variables|Default|GetCurrentRecoil)) 0.0) false false)
      (Variables|Default|SetCurrentRecoil (Math|Interpolation|FInterptoConstant (Variables|Default|GetCurrentRecoil) 0.0 Time (.RecoilDropSpeed (Utilities|Struct|BreakWeaponStructure (Variables|/Game/All/Blueprints/Weapon/Weapon.Weapon_C|GetConfig _weapon)))))
      (else
        (Variables|/Game/All/Blueprints/Weapon/Weapon.Weapon_C|SetTrackIndex _weapon 0.0)))))

(fn Stoplmm
  (params (Key :type Key%20Structure :default "None"))
  (bind _returnvalue (Transformation|GetVelocity))
  (bind _returnvalue_2 (Transformation|GetActorRotation))
  (bind _returnvalue_3 (Math|Vector|GetForwardVector _returnvalue_2))
  (bind _returnvalue_4 (Math|Vector|GetRightVector _returnvalue_2))
  (Utilities|FlowControl|Sequence
    (:then_0
      (LocalVariables|SetSelfForward _returnvalue_3)
      (LocalVariables|SetSelfRight _returnvalue_4)
      (LocalVariables|SetHVelocity (Math|Vector|ProjectVectorontoPlane _returnvalue _returnvalue_3))
      (LocalVariables|SetVVelocity (Math|Vector|ProjectVectorontoPlane _returnvalue _returnvalue_4)))
    (:then_1
      (if (== Key "W")
        (if (< (Math|Vector|DotProduct (LocalVariables|GetSelfForward) (LocalVariables|GetVVelocity)) 0.0)
          (Variables|/Script/Engine.MovementComponent|SetVelocity (Variables|Character|GetCharacterMovement) (LocalVariables|GetHVelocity))
          (Variables|Default|SetStopper 0.0 :!label _label)
          (CallFunction|RecoverStopper))))
    (:then_2
      (if (== Key "S")
        (if (> (Math|Vector|DotProduct (LocalVariables|GetSelfForward) (LocalVariables|GetVVelocity)) 0.0)
          (Variables|/Script/Engine.MovementComponent|SetVelocity (Variables|Character|GetCharacterMovement) (LocalVariables|GetHVelocity))
          (goto _label))))
    (:then_3
      (if (== Key "A")
        (if (> (Math|Vector|DotProduct (LocalVariables|GetSelfRight) (LocalVariables|GetHVelocity)) 0.0)
          (Variables|/Script/Engine.MovementComponent|SetVelocity (Variables|Character|GetCharacterMovement) (LocalVariables|GetVVelocity))
          (goto _label))))
    (:then_4
      (if (== Key "D")
        (if (< (Math|Vector|DotProduct (LocalVariables|GetSelfRight) (LocalVariables|GetHVelocity)) 0.0)
          (Variables|/Script/Engine.MovementComponent|SetVelocity (Variables|Character|GetCharacterMovement) (LocalVariables|GetVVelocity))
          (goto _label))))))

(fn GetCamera
  (return (Variables|Default|GetCamera) (Variables|Default|GetCameraOrigin)))

(fn OnDie
  (bind _weapon (CallFunction|GetCurrentWeapon))
  (bind _shooterui (Variables|Default|GetShooterUI))
  (bind _crcsshairui (Variables|/Game/All/Blueprints/Weapon/Weapon.Weapon_C|GetCrcsshairUI _weapon))
  (|CallParentFunction)
  (Utilities|FlowControl|Sequence
    (:then_0
      (Networking|SwitchHasAuthority
        (:Authority
          (CallFunction|EventonDie))))
    (:then_1
      ;[1 1 1] 清空准星
      (if (Pawn|IsLocallyControlled)
        (Utilities|FlowControl|Sequence
          (:then_0
            (Utilities|IsValid _crcsshairui
              (:Is%20Valid
                (Widget|RemovefromParent _crcsshairui))))
          (:then_1
            (Utilities|IsValid _shooterui
              (:Is%20Valid
                (Widget|RemovefromParent _shooterui)))))))))