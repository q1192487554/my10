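; Base shooter character that manages a networked weapon inventory with one slot per weapon type, plus Health, with stubbed aim, camera and shot hooks.
; The server spawns a starting Knife, set up through a RepNotify, applies damage, and broadcasts sphere-overlap auto-pickups.
; Equipping attaches to the local or third-person mesh, with remotes repeating the delayed attach.
; Dropping equips a nearby same-type weapon or falls back to slot 3.
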(event OnComponentBeginOverlap(Sphere)
  (params (OverlappedComponent :type Primitive%20Component%20Object%20Reference) (OtherActor :type Actor%20Object%20Reference) (OtherComp :type Primitive%20Component%20Object%20Reference) (OtherBodyIndex :type Integer) (bFromSweep :type Boolean) (SweepResult :type Hit%20Result%20Structure%20%28by%20ref%29))
  ;[1 1 1] 自动捡枪
  (Networking|SwitchHasAuthority
    (:Authority
      (bind _asweapon (Utilities|Casting|CastToWeapon OtherActor))
      (if (and (== (Utilities|Array|Get(acopy) (Variables|Default|GetWeaponArray) (Default|GetType _asweapon)) 0) (not (Default|HasOwner _asweapon)))
        (CallFunction|All-PickupWeapon _asweapon)))))

(event Custom|All-PickupWeapon
  (params (Weapon :type Weapon%20Object%20Reference))
  ;[1 1 1] 自动捡枪
  ;;[1 1 1] 服务器广播捡枪
  (CallFunction|PickWeapon Weapon))

(event Custom|AttachWeapon
  (params (WeaponIndex :type Integer))
  (bind _mesh (CallFunction|GetMash))
  (bind _weaponarray (Variables|Default|GetWeaponArray))
  (bind _output (Utilities|Array|Get(acopy) _weaponarray WeaponIndex))
  ;[1 1 1] 把枪放到角色骨骼上去
  (Networking|SwitchHasAuthority
    (:Authority
      (Transformation|AttachComponentToComponent _output _mesh "b_RightWeaponSocket" "SnapToTarget" "SnapToTarget" "SnapToTarget" true))
    (:Remote
      (Utilities|FlowControl|Sequence
        (:then_0
          (goto _label Reset))
        (:then_1
          (Utilities|FlowControl|DoN 10 :!label _label
            (:Exit
              (Utilities|FlowControl|Delay 0.1)
              (Transformation|AttachComponentToComponent _output _mesh "b_RightWeaponSocket" "SnapToTarget" "SnapToTarget" "SnapToTarget" true)
              (goto _label))))))))

(event EventBeginPlay
  (CallFunction|CreateWeapon "/Game/All/Blueprints/Weapon/Knife.Knife_C"))

(event Collision|EventActorBeginOverlap
  (params (OtherActor :type Actor%20Object%20Reference)))

(event EventTick
  (params (DeltaSeconds :type Float%20%28single-precision%29)))

(fn ConstructionScript)

(fn CreateWeapon
  (params (WeaponClass :type Weapon%20Class%20Reference))
  (Networking|SwitchHasAuthority
    (:Authority
      (bind _returnvalue (Game|SpawnActorfromClass WeaponClass (Math|Transform|MakeTransform "0, 0, 0" "0, 0, 0" "1,1,1") "Undefined" 0 0))
      (Variables|Default|SetWeaponCreated _returnvalue))))

(fn GetShootStartPosition
  (return "0, 0, 0"))

(fn GetShootDirection
  (return "0, 0, 0"))

(fn OnShootOnce
  (params (Recoil :type Float%20%28single-precision%29)))

(fn GetCurrentWeapon
  (return (Utilities|Array|Get(acopy) (Variables|Default|GetWeaponArray) (Variables|Default|GetCurrentWeaponIndex))))

(fn SetCurrentWeapon
  (params (Weapon :type Weapon%20Object%20Reference))
  (bind _weapon (CallFunction|GetCurrentWeapon))
  (Utilities|FlowControl|Sequence
    (:then_0
      ;[1 1 1] 隐藏上个抢 并且执行他的销毁函数
      (Utilities|IsValid _weapon
        (:Is%20Valid
          (CallFunction|SetVisibility _weapon false)
          (Default|OnUnEquIp _weapon))))
    (:then_1
      ;[1 1 1] 上一个抢index
      (Variables|Default|SetLastWeaponIndex (Variables|Default|GetCurrentWeaponIndex)))
    (:then_2
      ;[1 1 1] 显示当前抢
      (Variables|Default|SetCurrentWeaponIndex (Default|GetType Weapon))
      (CallFunction|SetVisibility Weapon true))
    (:then_3
      ;[1 1 1] 调用枪EquIp函数
      (Default|OnEquIp Weapon))))

(fn SwitchWeapon
  (params (Index :type Integer) (ResetCurrentGun :type Boolean))
  (LocalVariables|SetIsResetCurrentGun ResetCurrentGun)
  (if (and (!= Index (Variables|Default|GetCurrentWeaponIndex)) (!= (Utilities|Array|Get(acopy) (Variables|Default|GetWeaponArray) Index) 0))
    (Utilities|FlowControl|Sequence
      (:then_0
        (if (LocalVariables|GetIsResetCurrentGun)
          (CallFunction|ResetCurrentGun)))
      (:then_1
        (CallFunction|EquipWeapon Index)))))

(fn DropWeapon
  (bind _weapon (CallFunction|GetCurrentWeapon))
  (if (!= (Variables|Default|GetCurrentWeaponIndex) 3)
    (Utilities|FlowControl|Sequence
      (:then_0
        (CallFunction|ResetCurrentGun))
      (:then_1
        (Transformation|DetachFromActor _weapon "KeepWorld" "KeepWorld" "KeepWorld")
        (LocalVariables|SetDroppingWeapon _weapon))
      (:then_2
        (Default|OnDrop (CallFunction|GetCurrentWeapon) (* (Math|Vector|GetForwardVector (Transformation|GetActorRotation)) 1e+03)))
      (:then_3
        (Utilities|Array|SetArrayElem (Variables|Default|GetWeaponArray) (Variables|Default|GetCurrentWeaponIndex) 0))
      (:then_4
        (bind _output_get (LocalVariables|SetNextWeapon (CallFunction|GetNearbyWeapon (Variables|Default|GetCurrentWeaponIndex) (LocalVariables|GetDroppingWeapon))))
        (if (== _output_get 0)
          (CallFunction|SwitchWeapon 3 false)
          (Variables|Default|SetLastWeaponIndex 3)
          (else
            (CallFunction|PickWeapon _output_get)))))))

(fn PickWeapon
  (params (Weapon :type Weapon%20Object%20Reference))
  (bind _type (Default|GetType Weapon))
  (Utilities|FlowControl|Sequence
    (:then_0
      (Utilities|Array|SetArrayElem (Variables|Default|GetWeaponArray) _type Weapon))
    (:then_1
      (Default|OnPick Weapon self))
    (:then_2
      (CallFunction|EquipWeapon _type))))

(fn GetNearbyWeapon
  (params (Index :type Integer) (ExceptThis :type Weapon%20Object%20Reference))
  (for _array_element (Collision|GetOverlappingActors (Variables|Default|GetSphere) "/Game/All/Blueprints/Weapon/Weapon.Weapon_C" :!class /Script/Engine.PrimitiveComponent)
    (if (Math|Boolean|ANDBoolean (== Index (Default|GetType (.AsWeapon (Utilities|Casting|CastToWeapon _array_element)))) (not (Default|HasOwner (.AsWeapon (Utilities|Casting|CastToWeapon _array_element)))) (!= (.AsWeapon (Utilities|Casting|CastToWeapon _array_element)) ExceptThis))
      (return (.AsWeapon (Utilities|Casting|CastToWeapon _array_element))))))

(fn EquipWeapon
  (params (Index :type Integer))
  (bind _weaponarray (Variables|Default|GetWeaponArray))
  (bind _output (Utilities|Array|Get(acopy) _weaponarray Index))
  (Utilities|FlowControl|Sequence
    (:then_0
      ;[1 1 1] 把枪放到角色骨骼上去
      (CallFunction|AttachWeapon Index))
    (:then_1
      (CallFunction|SetCurrentWeapon _output))
    (:then_2
      (Default|PlayMontage _output "NewEnumerator2"))))

(fn GetCamera
  (return 0 0))

(fn ResetCurrentGun
  ;[1 1 1] 先让当前枪恢复默认状态
  (Default|Reset (CallFunction|GetCurrentWeapon)))

(fn OnRepWeaponCreated
  (bind _weaponcreated (Variables|Default|GetWeaponCreated))
  (Utilities|FlowControl|Sequence
    (:then_0
      ;[1 1 1] 处理碰撞
      (Collision|SetActorEnableCollision (Variables|Default|GetWeaponCreated) false)
      (Development|PrintString "Hello"))
    (:then_1
      (Utilities|Array|SetArrayElem (Variables|Default|GetWeaponArray) (Default|GetType _weaponcreated) _weaponcreated))
    (:then_2
      (Transformation|AttachComponentToComponent (Variables|Default|GetWeaponCreated) (CallFunction|GetMash) "b_RightWeaponSocket" "SnapToTarget" "SnapToTarget" "SnapToTarget" true))
    (:then_3
      (Default|SetWeaponOwner (Variables|Default|GetWeaponCreated) self))
    (:then_4
      (CallFunction|SetVisibility (Variables|Default|GetWeaponCreated) false))
    (:then_5
      (CallFunction|SetCurrentWeapon (Variables|Default|GetWeaponCreated)))
    (:then_6
      (return))))

(fn TakeDamage
  (params (Damage :type Float%20%28single-precision%29))
  (Networking|SwitchHasAuthority
    (:Authority
      (if (> (Variables|Default|GetHealth) 0.0)
        (Variables|Default|SetHealth (- (Variables|Default|GetHealth) Damage))))))

(fn GetMash
  (if (Pawn|IsLocallyControlled)
    (return (Variables|Character|GetMesh))
    (else
      (return (Variables|Default|GetTppMesh)))))