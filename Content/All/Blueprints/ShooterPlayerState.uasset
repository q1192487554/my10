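; ShooterPlayerState is a player state that gives each player a random name and relays chat messages.
; On BeginPlay the authority sets Name to a random three-digit number.
; Server-SendMessage forwards text to All-SendMessage, which passes it with Name to the first top-level ChatBoard widget, skipping dedicated servers.
; A delayed block that creates the local player's ChatBoard is disconnected and never runs.
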(event Custom|Server-SendMessage
  (params (Massage :type Text))
  (CallFunction|All-SendMessage Massage))

(event Custom|All-SendMessage
  (params (Massage :type Text))
  (if (not (Networking|IsDedicatedServer))
    (bind _foundwidgets (Widget|GetAllWidgetsOfClass "/Game/All/UMG/Widgets/Chat/ChatBoard.ChatBoard_C" true))
    (Default|OnMessageReceived (Utilities|Array|Get(acopy) _foundwidgets) Massage (Variables|Default|GetName))))

(event EventBeginPlay
  (Utilities|FlowControl|Sequence
    (:then_0
      (Networking|SwitchHasAuthority
        (:Authority
          (Variables|Default|SetName (Utilities|Text|ToText(Integer) (Math|Random|RandomIntegerinRange 100 999))))))))

(event EventTick
  (params (DeltaSeconds :type Float%20%28single-precision%29)))

(fn ConstructionScript)