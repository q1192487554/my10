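; AUG weapon Blueprint that adds a toggled scope zoom to its parent weapon class and supplies its own fire sound.
; Aim input steps a ZoomState machine that ignores presses mid-transition, plays zoom sounds and removes the crosshair on zoom-in.
; The ChangeCamera timeline plays forward or backward to blend the owner's camera position and FOV, reattaching it to the scope point or camera origin.
; A successful reload calls Reset, instantly restoring default FOV, attachment and zoom state.
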(event Custom|Event_OnAimButtonDown
  (bind _weaponowner (Variables|Default|GetWeaponOwner))
  (bind _weaponowner_2 (Variables|Default|GetWeaponOwner))
  (bind _crcsshairui (Variables|Default|GetCrcsshairUI))
  (bind (_camera _cameraorigin) (Default|GetCamera _weaponowner))
  (bind (_camera_2 _cameraorigin_2) (Default|GetCamera _weaponowner_2))
  (switch int (Variables|Default|GetZoomState)
    (:0
      (Variables|Default|SetZoomState 1)
      (Audio|PlaySoundatLocation "/Game/more/Assets/Sound/aug_zoom_in.aug_zoom_in" (Transformation|GetActorLocation) "0, 0, 0" 1.0 1.0 0.0 0 0 0)
      (Utilities|IsValid _crcsshairui
        (:Is%20Valid
          (Widget|RemovefromParent _crcsshairui)
          (bind (_direction _alphf) (Timeline|ChangeCamera PlayFromStart)
            (:Update
              ;[1 1 1] 设置镜头位置
              (Transformation|SetWorldLocation _camera_2 (Math|Vector|Lerp(Vector) (Transformation|GetWorldLocation _cameraorigin_2) (Transformation|GetWorldLocation (Variables|Default|GetCameraPoint)) _alphf) false false)
              ;[1 1 1] 设置缩放
              (Camera|SetFieldOfView (.Camera (Default|GetCamera (Variables|Default|GetWeaponOwner))) (Math|Float|Lerp 9e+01 4e+01 _alphf)))
            (:Finished
              ;[1 1 1] 动画播放完毕判断是正向还是反向
              (switch Utilities|FlowControl|Switch|SwitchonETimelineDirection _direction
                (:Forward
                  (Variables|Default|SetZoomState 2)
                  (Transformation|AttachComponentToComponent _camera (Variables|Default|GetCameraPoint) "None" "KeepWorld" "KeepWorld" "KeepWorld" true))
                (:Backward
                  (Variables|Default|SetZoomState 0)
                  (Transformation|AttachComponentToComponent _camera _cameraorigin "None" "SnapToTarget" "SnapToTarget" "SnapToTarget" true))))))
        (:Is%20Not%20Valid
          (Timeline|ChangeCamera PlayFromStart))))
    (:2
      (Variables|Default|SetZoomState 3)
      (Audio|PlaySoundatLocation "/Game/more/Assets/Sound/aug_zoom_out.aug_zoom_out" (Transformation|GetActorLocation) "0, 0, 0" 1.0 1.0 0.0 0 0 0)
      (CallFunction|SetDefault)
      (Timeline|ChangeCamera ReverseFromEnd))))

(event EventBeginPlay
  (|CallParentFunction) ; 此节点被禁用，将不会被调用。\n从引脚连出引线来编译功能。
)

(event Collision|EventActorBeginOverlap
  (params (OtherActor :type Actor%20Object%20Reference))
  (|CallParentFunction OtherActor) ; 此节点被禁用，将不会被调用。\n从引脚连出引线来编译功能。
)

(event EventTick
  (params (DeltaSeconds :type Float%20%28single-precision%29))
  (|CallParentFunction DeltaSeconds) ; 此节点被禁用，将不会被调用。\n从引脚连出引线来编译功能。
)

(fn ConstructionScript
  (|CallParentFunction))

(fn OnAimButtonDown
  (|CallParentFunction)
  (CallFunction|EventonAimButtonDown))

(fn Reset
  (bind _weaponowner (Variables|Default|GetWeaponOwner))
  (bind (_camera _cameraorigin) (Default|GetCamera _weaponowner))
  (|CallParentFunction)
  (Utilities|FlowControl|Sequence
    (:then_0
      (Camera|SetFieldOfView (.Camera (Default|GetCamera (Variables|Default|GetWeaponOwner))) 9e+01))
    (:then_1
      (Variables|Default|SetZoomState 0)
      (Transformation|AttachComponentToComponent _camera _cameraorigin "None" "SnapToTarget" "SnapToTarget" "SnapToTarget" true))))

(fn OnReloadButtonDown
  (bind _ismayreload (|CallParentFunction))
  (if _ismayreload
    (CallFunction|Reset)))

(fn GetFireSound
  (return "/Game/more/Assets/Sound/aug-1.aug-1"))

(fn OnDrop
  (params (Force :type Vector :default "0, 0, 0"))
  (|CallParentFunction Force))