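; Base weapon actor for shooters, handling firing, reloading, pickup/drop physics and a local crosshair widget.
; Stats load from a data table row named after the class, selecting auto or single fire and montage sets.
; Instant shots line-trace to apply damage, impulses and decals; projectile firing is an empty stub.
; A decaying buffer absorbs recoil before passing excess to the owner, whose recoil widens spread and drives sine-wave yaw drift.
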(event Custom|ShootInAuto
  (CallFunction|OnShootStartinAuto)
  (蒙太奇|PlayMontage "NewEnumerator0")
  (Variables|Default|SetIsShootInAuto true)
  (CallFunction|ShootOnce :!label _label)
  (Utilities|FlowControl|Delay (获得配置|GetShootInterval))
  ;[1 1 1] 判断是否有子弹
  (if (获得状态|HasBulletinClip)
    ;[1 1 1] 是否在shoot Auto模式下射击
    (if (Variables|Default|GetIsShootInAuto)
      (goto _label))
    (else
      (CallFunction|ShootStop))))

(event Custom|IninEnd
  (Utilities|FlowControl|Delay 0.2)
  ;[1 1 1] 初始化模拟物理
  (Physics|SetSimulatePhysics (Variables|Default|GetRoot) (not (CallFunction|HasOwner))))

(event EventBeginPlay
  (CallFunction|IninEnd))

(event Collision|EventActorBeginOverlap
  (params (OtherActor :type Actor%20Object%20Reference)))

(event EventTick
  (params (DeltaSeconds :type Float%20%28single-precision%29))
  (Utilities|FlowControl|Delay 0.1)
  ;[1 1 1] 后坐力回退
  (CallFunction|RecoilKeptDrop DeltaSeconds))

(fn ConstructionScript
  (bind _config (Variables|Default|GetConfig))
  (bind (_price _type _auto _instant _clipsize _maxbulletnum) (Utilities|Struct|BreakWeaponStructure _config))
  (CallFunction|ReadConfig)
  (Variables|Default|SetBulletNum _clipsize)
  (Variables|Default|SetMaxBulletNum _maxbulletnum))

(fn ReadConfig
  (bind _returnvalue (Utilities|GetDataTableRow "/Game/All/Config/WeaponConfigTable.WeaponConfigTable" (Utilities|String|StringToName (CallFunction|GetClassName self)))
    (:then
      (Variables|Default|SetConfig _returnvalue))))

(fn GetAnimGroup
  (return (.AnimGroup (Utilities|Struct|BreakWeaponStructure (Variables|Default|GetConfig)))))

(fn OnShootButtonDown
  (if (not (CallFunction|IsReloading))
    (if (获得配置|IsAuto)
      (CallFunction|TryShootinAuto)
      (else
        (CallFunction|TryShootOnce)))))

(fn OnShootButtonUp
  (Utilities|FlowControl|Sequence
    (:then_0
      (if (Variables|Default|GetIsShootInAuto)
        (CallFunction|ShootStop)))
    (:then_1
      (if (not (> (Variables|Default|GetBulletNum) 0))
        (控制输入|OnReloadButtonDown)))))

(fn OnAimButtonDown)

(fn OnAimButtonUp)

(fn OnReloadButtonDown
  (if (not (Variables|Default|GetIsShootInAuto))
    (if (> (Variables|Default|GetMaxBulletNum) 0)
      (if (not (>= (Variables|Default|GetBulletNum) (获得配置|GetClipSize)))
        (if (not (CallFunction|IsReloading))
          (蒙太奇|PlayMontage "NewEnumerator1")
          (Utilities|Time|SetTimerbyFunctionName 0 "ReloadOver" (获得配置|GetReloadTime))
          (Variables|Default|SetLastReloadTime (Utilities|Time|GetTimeSeconds))
          (return true))))))

(fn OnReloadButtonUp)

(fn IsAuto
  (return (.Auto (Utilities|Struct|BreakWeaponStructure (Variables|Default|GetConfig)))))

(fn TryShootinAuto
  (if (not (Variables|Default|GetIsShootInAuto))
    ;[1 1 1] 检查弹夹是否有子弹
    (if (获得状态|HasBulletinClip)
      (CallFunction|ShootinAuto))))

(fn TryShootOnce
  (if (获得状态|HasBulletinClip)
    (if (not (CallFunction|IsinCD))
      (CallFunction|ShootOnce)
      (蒙太奇|PlayMontage "NewEnumerator0"))))

(fn HasBulletinClip
  (return (> (Variables|Default|GetBulletNum) 0)))

(fn ShootOnce
  ;[1 1 1] 开抢声音
  (Audio|PlaySoundatLocation (声音|GetFireSound) (Transformation|GetActorLocation self) "0, 0, 0" 1.0 1.0 0.0 0 0 0)
  (Variables|Default|SetLastShootTime (Utilities|Time|GetTimeSeconds))
  (Math|Integer|DecrementInt (Variables|Default|GetBulletNum)
    (:%20%20
      ;[1 1 1] 判断是不是瞬时子弹
      (if (获得配置|IsInstant)
        (CallFunction|ShootInstant)
        (else
          (CallFunction|ShootProjectile)))
      (CallFunction|FeedRecoin))))

(fn GetShootInterval
  (return (.ShootInterval (Utilities|Struct|BreakWeaponStructure (Variables|Default|GetConfig)))))

(fn IsInstant
  (return (.Instant (Utilities|Struct|BreakWeaponStructure (Variables|Default|GetConfig)))))

(fn ShootInstant
  (bind (_position _direction) (CallFunction|ConmputeShooteEndPosition))
  ;[1 1 1] 射线追踪
  (bind (_outhit _returnvalue) (Collision|LineTraceByChannel (Default|GetShootStartPosition (Variables|Default|GetWeaponOwner)) _position "TraceTypeQuery2" false (Utilities|Array|MakeArray (Variables|Default|GetWeaponOwner)) "None"))
  (if _returnvalue
    (Utilities|FlowControl|Sequence
      (:then_0
        (CallFunction|GenerateTrace (.ImpactPoint (Collision|BreakHitResult _outhit)) (.ImpactNormal (Collision|BreakHitResult _outhit)))
        ;[1 1 1] 判断集中的内容有移动属性的话给他加一个力
        (if (and (Utilities|Enum|Equal(Enum) (Variables|/Script/Engine.SceneComponent|GetMobility (.HitComponent (Collision|BreakHitResult _outhit))) "Movable") (Physics|IsSimulatingPhysics (.HitComponent (Collision|BreakHitResult _outhit)) "None"))
          (Physics|AddImpulse (.HitComponent (Collision|BreakHitResult _outhit)) (* _direction 2e+03) "None" false)))
      (:then_1
        (bind _asshooter (Utilities|Casting|CastToShooter (.HitActor (Collision|BreakHitResult _outhit))))
        (Default|TakeDamage _asshooter 2e+01)))))

(fn ShootProjectile)

(fn ConmputeShooteEndPosition
  (bind _direction (CallFunction|GetShootDirection))
  (return (+ (Default|GetShootStartPosition (Variables|Default|GetWeaponOwner)) (* _direction (获得配置|GetEffectiveRange))) _direction))

(fn GetShootDirection
  (bind _weaponowner (Variables|Default|GetWeaponOwner))
  (bind _weaponowner_2 (Variables|Default|GetWeaponOwner))
  (bind _direction (Default|GetShootDirection _weaponowner_2))
  (bind _currentrecoil (Variables|/Game/All/Blueprints/Character/Shooter.Shooter_C|GetCurrentRecoil _weaponowner))
  (return (Class|KismetMathLibrary|RandomUnitVectorinConeinRadians (Math|Vector|GetForwardVector (Math|Rotator|MakeRotator (.roll _direction) (+ (.pitch _direction) _currentrecoil) (+ (.yaw _direction) (CallFunction|ComputeTrackOffset)))) (/ (* (Variables|Default|GetRadius) (/ (+ _currentrecoil 2.0) 2.0)) (获得配置|GetAccurateRange)))))

(fn GetAccurateRange
  (return (.AccurateRange (Utilities|Struct|BreakWeaponStructure (Variables|Default|GetConfig)))))

(fn SetWeaponOwner
  (params (Shooter :type Shooter%20Object%20Reference))
  (Variables|Default|SetWeaponOwner Shooter))

(fn ShootStop
  (Variables|Default|SetIsShootInAuto false)
  (蒙太奇|StopMontage "NewEnumerator0")
  (CallFunction|OnShootStopinAuto))

(fn IsinCD
  (return (> (+ (Variables|Default|GetLastShootTime) (获得配置|GetShootInterval)) (Utilities|Time|GetTimeSeconds))))

(fn PlayMontage
  (params (ActionEnum :type ActionEnum%20Enum :default "NewEnumerator0"))
  (Animation|PlayAnimMontage (Variables|Default|GetWeaponOwner) (蒙太奇|GetMontage ActionEnum) 1.0 "None"))

(fn GetMontage
  (params (ActionEnum :type ActionEnum%20Enum :default "NewEnumerator0"))
  (switch int (获得配置|GetAnimGroup)
    (:0
      (switch Utilities|FlowControl|Switch|SwitchonActionEnum ActionEnum
        (:NewEnumerator0
          (return "/Game/All/Assets/Montage/RifleFire_Montage.RifleFire_Montage"))
        (:NewEnumerator1
          (return "/Game/All/Assets/Montage/RifleReload_Montage.RifleReload_Montage"))
        (:NewEnumerator2
          (return "/Game/All/Assets/Montage/RifleEquip_Montage.RifleEquip_Montage"))))
    (:1
      (switch Utilities|FlowControl|Switch|SwitchonActionEnum ActionEnum
        (:NewEnumerator0
          (return "/Game/All/Assets/Montage/LauncherFire_Montage.LauncherFire_Montage"))
        (:NewEnumerator1
          (return "/Game/All/Assets/Montage/LauncherReload_Montage.LauncherReload_Montage"))
        (:NewEnumerator2
          (return "/Game/All/Assets/Montage/LauncherEquip_Montage.LauncherEquip_Montage"))))
    (:2
      (switch Utilities|FlowControl|Switch|SwitchonActionEnum ActionEnum
        (:NewEnumerator0
          (return "/Game/All/Assets/Montage/KnifeFire_Montage.KnifeFire_Montage"))
        (:NewEnumerator2
          (return "/Game/All/Assets/Montage/RifleEquip_Montage.RifleEquip_Montage"))))))

(fn StopMontage
  (params (ActionEnum :type ActionEnum%20Enum :default "NewEnumerator0"))
  (Animation|StopAnimMontage (Variables|Default|GetWeaponOwner) (蒙太奇|GetMontage ActionEnum)))

(fn GetClipSize
  (return (.ClipSize (Utilities|Struct|BreakWeaponStructure (Variables|Default|GetConfig)))))

(fn IsReloading
  (return (> (+ (Variables|Default|GetLastReloadTime) (获得配置|GetReloadTime)) (Utilities|Time|GetTimeSeconds))))

(fn GetReloadTime
  (return (.ReloadTime (Utilities|Struct|BreakWeaponStructure (Variables|Default|GetConfig)))))

(fn ReloadOver
  (Utilities|FlowControl|Sequence
    (:then_0
      (LocalVariables|SetEmptyNum (- (获得配置|GetClipSize) (Variables|Default|GetBulletNum))))
    (:then_1
      (if (< (+ (Variables|Default|GetMaxBulletNum) (Variables|Default|GetBulletNum)) (获得配置|GetClipSize))
        (Variables|Default|SetBulletNum (+ (Variables|Default|GetMaxBulletNum) (Variables|Default|GetBulletNum)))
        (else
          (Variables|Default|SetBulletNum (获得配置|GetClipSize)))))
    (:then_2
      (bind _output_get (Variables|Default|SetMaxBulletNum (- (Variables|Default|GetMaxBulletNum) (LocalVariables|GetEmptyNum))))
      (if (< _output_get 0)
        (Variables|Default|SetMaxBulletNum 0)))))

(fn OnShootStartinAuto)

(fn OnShootStopinAuto)

(fn GetDecalSize
  (return (.DecalSize (Utilities|Struct|BreakWeaponStructure (Variables|Default|GetConfig)))))

(fn GenerateTrace
  (params (Position :type Vector) (Direction :type Vector))
  (bind _decalsize (获得配置|GetDecalSize))
  (bind _returnvalue (Math|Conversions|RotationFromXVector Direction))
  (bind _returnvalue_2 (Rendering|Decal|SpawnDecalatLocation "/Game/Assets/Effects/Materials/Weapon/M_Impact_Decal.M_Impact_Decal" (Math|Vector|MakeVector _decalsize _decalsize _decalsize) Position (Math|Rotator|MakeRotator (Math|Random|RandomFloatinRange -1.8e+02 1.8e+02) (.pitch _returnvalue) (.yaw _returnvalue)) 5.0))
  ;[1 1 1] 设置贴纸可见距离
  (Rendering|Components|Decal|SetFadeScreenSize _returnvalue_2 0.0))

(fn GetMoveSpeed
  (return (.MoveSpeed (Utilities|Struct|BreakWeaponStructure (Variables|Default|GetConfig)))))

(fn ComputeTrackOffset
  (bind _output_get (Variables|Default|SetTrackIndex (+ (Variables|Default|GetTrackIndex) (* (Math|Float|Square (/ (Variables|/Game/All/Blueprints/Character/Shooter.Shooter_C|GetCurrentRecoil (Variables|Default|GetWeaponOwner)) (获得配置|GetMaxRecoil))) (Variables|Default|GetTrackFactor)))))
  (return (* (Math|Trig|Sin(Radians) _output_get) (.TrackOffset (Utilities|Struct|BreakWeaponStructure (Variables|Default|GetConfig))) -1.0)))

(fn GetMaxRecoil
  (return (.MaxRecoil (Utilities|Struct|BreakWeaponStructure (Variables|Default|GetConfig)))))

(fn FeedRecoin
  (bind _recoil (CallFunction|ConsumeRecoil))
  (if (> _recoil 0.0)
    (Default|OnShootOnce (Variables|Default|GetWeaponOwner) _recoil)))

(fn ConsumeRecoil
  (bind _output_get (LocalVariables|SetTargetRecoilKept (Math|Float|Min(Float) (+ (Variables|Default|GetRecoilKept) (获得配置|GetRecoil)) (获得配置|GetRecoilConsume))))
  (LocalVariables|SetRetValue (- (获得配置|GetRecoil) (- _output_get (Variables|Default|GetRecoilKept))))
  (Variables|Default|SetRecoilKept (LocalVariables|GetTargetRecoilKept))
  (return (LocalVariables|GetRetValue)))

(fn GetRecoil
  (return (.Recoil (Utilities|Struct|BreakWeaponStructure (Variables|Default|GetConfig)))))

(fn GetRecoilConsume
  (return (.RecoilConsume (Utilities|Struct|BreakWeaponStructure (Variables|Default|GetConfig)))))

(fn RecoilKeptDrop
  (params (Time :type Float%20%28single-precision%29))
  (if (> (Variables|Default|GetRecoilKept) 0.0)
    (Variables|Default|SetRecoilKept (Math|Interpolation|FInterptoConstant (Variables|Default|GetRecoilKept) 0.0 Time (获得配置|GetRecoilDropSpeed)))))

(fn GetRecoilDropSpeed
  (return (.RecoilDropSpeed (Utilities|Struct|BreakWeaponStructure (Variables|Default|GetConfig)))))

(fn GetFireSound
  (return 0))

(fn GetEffectiveRange
  (return (.EffectiveRange (Utilities|Struct|BreakWeaponStructure (Variables|Default|GetConfig)))))

(fn GetType
  (return (.Type (Utilities|Struct|BreakWeaponStructure (Variables|Default|GetConfig)))))

(fn OnEquIp
  (CallFunction|SetDefault))

(fn OnUnEquIp
  (Utilities|IsValid (Variables|Default|GetCrcsshairUI)
    (:Is%20Valid
      (Widget|RemovefromParent (Variables|Default|GetCrcsshairUI))
      (Variables|Default|SetCrcsshairUI 0))))

(fn OnDrop
  (params (Force :type Vector))
  (bind _returnvalue (Actor|GetComponentbyClass "/Script/Engine.MeshComponent"))
  (Utilities|FlowControl|Sequence
    (:then_0
      ;[1 1 1] 清空持枪者
      (Variables|Default|SetWeaponOwner 0))
    (:then_1
      (Collision|SetActorEnableCollision true)
      (Physics|SetSimulatePhysics _returnvalue true)
      (Physics|AddImpulse _returnvalue Force "None" false))
    (:then_2
      ;[1 1 1] 清空准星
      (生命周期|OnUnEquIp))))

(fn HasOwner
  (return (!= (Variables|Default|GetWeaponOwner) 0)))

(fn OnPick
  (params (Shooter :type Shooter%20Object%20Reference))
  (Utilities|FlowControl|Sequence
    (:then_0
      (Variables|Default|SetWeaponOwner Shooter))
    (:then_1
      ;[1 1 1] 取消碰撞
      (Collision|SetActorEnableCollision false))
    (:then_2
      ;[1 1 1] 模拟物理取消
      (Physics|SetSimulatePhysics (Actor|GetComponentbyClass "/Script/Engine.MeshComponent") false))))

(fn Reset)

(fn SetDefault
  (bind _returnvalue (Utilities|String|MakeLiteralString "Crcsshair_"))
  (bind _self self)
  (bind _name (CallFunction|GetClassName _self))
  (bind _returnvalue_2 (Utilities|String|Append _returnvalue _name))
  (bind _class (CallFunction|GetUserWidgetbyName _returnvalue_2))
  (if (Pawn|IsLocallyControlled (Variables|Default|GetWeaponOwner))
    (if (!= _class 0)
      (bind _ui (CallFunction|CreateWidgetandAddtoViewport _class))
      (Variables|Default|SetCrcsshairUI _ui))))