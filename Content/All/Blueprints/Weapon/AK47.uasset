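; AK47 is a weapon Blueprint that supplies the rifle's automatic-fire effects and firing sound on top of its parent weapon class.
; When auto shooting starts, it attaches an assault rifle muzzle flash emitter to the Arrow component and stores it in FireEffects.
; When shooting stops, it destroys that emitter if still valid.
; GetFireSound returns the AK47 sound, while BeginPlay and construction only call the parent.
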(event EventBeginPlay
  (|CallParentFunction))

(event Collision|EventActorBeginOverlap
  (params (OtherActor :type Actor%20Object%20Reference))
  (|CallParentFunction OtherActor) ; 此节点被禁用，将不会被调用。\n从引脚连出引线来编译功能。
)

(event EventTick
  (params (DeltaSeconds :type Float%20%28single-precision%29))
  (|CallParentFunction DeltaSeconds) ; 此节点被禁用，将不会被调用。\n从引脚连出引线来编译功能。
)

(fn ConstructionScript
  (|CallParentFunction))

(fn OnShootStartinAuto
  (|CallParentFunction)
  (bind _returnvalue (Effects|SpawnEmitterAttached "/Game/Assets/Effects/ParticleSystems/Weapons/AssaultRifle/Muzzle/P_AssaultRifle_MF.P_AssaultRifle_MF" (Variables|Default|GetArrow) "None"))
  (Variables|Default|SetFireEffects _returnvalue))

(fn OnShootStopinAuto
  (bind _fireeffects (Variables|Default|GetFireEffects))
  (|CallParentFunction)
  (Utilities|IsValid _fireeffects
    (:Is%20Valid
      (Components|DestroyComponent _fireeffects))))

(fn GetFireSound
  (return "/Game/Assets/Sound/ak47_01.ak47_01"))