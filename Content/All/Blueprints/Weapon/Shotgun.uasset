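; Shotgun weapon Blueprint, a child of a parent weapon class, with XM1014 fire and pump sounds.
; Its ShootInstant override runs the parent's instant shot ten times to fire ten pellets per shot, then calls the shoot-end event.
; That event waits briefly and plays the pump sound at the actor's location.
; GetFireSound supplies the shotgun's own firing sound.
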(event Custom|Event_ShootInstantEnd
  (Utilities|FlowControl|Delay 0.3)
  (Audio|PlaySoundatLocation "/Game/more/Assets/Sound/xm1014_pump.xm1014_pump" (Transformation|GetActorLocation) "0, 0, 0" 1.0 1.0 0.0 0 0 0))

(event EventBeginPlay
  (|CallParentFunction) ; 此节点被禁用，将不会被调用。\n从引脚连出引线来编译功能。
)

(event Collision|EventActorBeginOverlap
  (params (OtherActor :type Actor%20Object%20Reference))
  (|CallParentFunction OtherActor) ; 此节点被禁用，将不会被调用。\n从引脚连出引线来编译功能。
)

(event EventTick
  (params (DeltaSeconds :type Float%20%28single-precision%29))
  (|CallParentFunction DeltaSeconds) ; 此节点被禁用，将不会被调用。\n从引脚连出引线来编译功能。
)

(fn ConstructionScript
  (|CallParentFunction))

(fn ShootInstant
  ;[1 1 1] 10发子弹
  (for _index (range 0 9)
    (|CallParentFunction))
  (CallFunction|EventShootInstantEnd))

(fn GetFireSound
  (return "/Game/more/Assets/Sound/xm1014-1.xm1014-1"))