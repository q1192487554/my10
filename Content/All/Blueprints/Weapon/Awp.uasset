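; AWP sniper rifle weapon Blueprint that adds scoped aiming on top of its parent weapon class.
; The aim button cycles three zoom states, setting camera FOV for the local player and playing a sound when zoomed.
; Scoping hides the weapon and shows a crosshair widget whose blur is animated by a timeline.
; Shooting, reloading and unequipping call Reset, which restores FOV and visibility and removes the scope.
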(event Custom|Event_ChangeBlur_TimeLine
  (params (Crcsshair_AWP_Aim_UI :type Crcsshair%20AWP%20Aim%20Object%20Reference))
  ;[1 1 1] 处理开镜瞬间模糊
  (bind _blur (Timeline|ChangeBlur PlayFromStart)
    (:Update
      (CallFunction|SetAWPAimBlur _blur Crcsshair_AWP_Aim_UI))))

(event EventBeginPlay
  (|CallParentFunction) ; 此节点被禁用，将不会被调用。\n从引脚连出引线来编译功能。
)

(event Collision|EventActorBeginOverlap
  (params (OtherActor :type Actor%20Object%20Reference))
  (|CallParentFunction OtherActor) ; 此节点被禁用，将不会被调用。\n从引脚连出引线来编译功能。
)

(event EventTick
  (params (DeltaSeconds :type Float%20%28single-precision%29))
  (|CallParentFunction DeltaSeconds) ; 此节点被禁用，将不会被调用。\n从引脚连出引线来编译功能。
)

(fn ConstructionScript
  (|CallParentFunction))

(fn OnAimButtonDown
  (|CallParentFunction)
  (Utilities|FlowControl|Sequence
    (:then_0
      ;[1 1 1] 0 1 2 循环
      (bind _result (Math|Integer|IncrementInt (Variables|Default|GetZoomState))
        (:%20%20
          (bind _output_get (Variables|Default|SetZoomState (Math|Integer|%(Integer) _result 3)))
          ;[1 1 1] 实现 瞄准
          (if (Pawn|IsLocallyControlled (Variables|Default|GetWeaponOwner))
            (Camera|SetFieldOfView (.Camera (Default|GetCamera (Variables|Default|GetWeaponOwner))) (Utilities|Array|Get(acopy) (Variables|Default|GetZoomFOV) _output_get))))))
    (:then_1
      (if (Pawn|IsLocallyControlled (Variables|Default|GetWeaponOwner))
        (switch int (Variables|Default|GetZoomState)
          (:0
            ;[1 1 1] 关闭狙击准星要做的事情
            (CallFunction|SetVisibility self true)
            (Utilities|IsValid (Variables|Default|GetCrcsshairUI)
              (:Is%20Valid
                (Widget|RemovefromParent (Variables|Default|GetCrcsshairUI))
                (Variables|Default|SetCrcsshairUI 0))))
          (:1
            ;[1 1 1] 开启狙击准星要做的事情
            (CallFunction|SetVisibility self false)
            ;;[1 1 1] 添加 瞄准 ui
            (bind _ui (CallFunction|CreateWidgetandAddtoViewport "/Game/All/UI/Crcsshair/Crcsshair_AWP_Aim.Crcsshair_AWP_Aim_C" -1))
            (bind _output_get_2 (Variables|Default|SetCrcsshairUI _ui))
            (bind _ascrcsshair_awp_aim (Utilities|Casting|CastToCrcsshair_AWP_Aim _output_get_2))
            ;;[1 1 1] 处理模糊
            (CallFunction|EventChangeBlurTimeLine _ascrcsshair_awp_aim)))))
    (:then_2
      (switch int (Variables|Default|GetZoomState)
        (:1
          _)
        (:2
          _))
      ;[1 1 1] 狙击枪开镜声音
      (Audio|PlaySoundatLocation "/Game/Assets/Sound/zoom16.zoom16" (Transformation|GetActorLocation self) "0, 0, 0" 1.0 1.0 0.0 0 0 0))))

(fn SetAWPAimBlur
  (params (Blur :type Float%20%28single-precision%29) (Crcsshair_AWP_Aim_UI :type Crcsshair%20AWP%20Aim%20Object%20Reference))
  (Class|BackgroundBlur|SetBlurStrength (Variables|/Game/All/UI/Crcsshair/Crcsshair_AWP_Aim.Crcsshair_AWP_Aim_C|GetBlur Crcsshair_AWP_Aim_UI) Blur))

(fn GetFireSound
  (return "/Game/Assets/Sound/awp1.awp1"))

(fn ShootOnce
  (|CallParentFunction)
  (CallFunction|Reset))

(fn OnReloadButtonDown
  (|CallParentFunction)
  (CallFunction|Reset))

(fn OnUnEquIp
  (|CallParentFunction)
  (CallFunction|Reset))

(fn Reset
  (|CallParentFunction)
  (if (!= (Variables|Default|GetZoomState) 0)
    (Utilities|FlowControl|Sequence
      (:then_0
        ;[1 1 1] 相机恢复
        (Camera|SetFieldOfView (.Camera (Default|GetCamera (Variables|Default|GetWeaponOwner))) (Utilities|Array|Get(acopy) (Variables|Default|GetZoomFOV))))
      (:then_1
        (CallFunction|SetVisibility self true)
        (Variables|Default|SetZoomState 0))
      (:then_2
        ;[1 1 1] 删除瞄准镜
        (Utilities|IsValid (Variables|Default|GetCrcsshairUI)
          (:Is%20Valid
            (Widget|RemovefromParent (Variables|Default|GetCrcsshairUI))
            (Variables|Default|SetCrcsshairUI 0)))))))